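; Interaction component that lets the player interact with the object under the camera's view.
; Each Tick it runs a Visibility line trace from the player 0 camera out to InteractRange, with debug drawing on, and caches the hit actor if it implements BPI_Interactable, clearing it otherwise.
; The IA_Interact input's Triggered event sends OnInteractMessage to the cached actor when it is valid.
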(event Input|EnhancedActionEvents|EnhancedInputActionIA_Interact
  (params (ActionValue :type Boolean) (ElapsedSeconds :type Float%20%28double-precision%29) (TriggeredSeconds :type Float%20%28double-precision%29) (InputAction :type Input%20Action%20Object%20Reference :default "/Game/Input/Actions/IA_Interact.IA_Interact"))
  (:Triggered
    (bind _interactable_actor (Variables|Default|GetInteractable%20Actor)
      (:then
        (Class|BPIInteractable|OnInteract(Message) _interactable_actor))
      (:else))))

(event EventBeginPlay)

(event EventTick
  (params (DeltaSeconds :type Float%20%28single-precision%29))
  (bind _returnvalue (Game|GetPlayerCameraManager 0))
  (bind _returnvalue_2 (Camera|GetCameraLocation _returnvalue))
  (bind _outhit (Collision|LineTraceByChannel _returnvalue_2 (+ _returnvalue_2 (* (Transformation|GetActorForwardVector _returnvalue) (Variables|Default|GetInteract%20Range))) "TraceTypeQuery1" false 0 "ForOneFrame"))
  (if (.bblockinghit _outhit)
    (if (Utilities|DoesObjectImplementInterface (.hitactor _outhit) "/Game/Blueprints/interaction/_BPI_Interactable._BPI_Interactable_C")
      (Variables|Default|SetInteractable%20Actor (.hitactor _outhit))
      (else
        (Variables|Default|SetInteractable%20Actor 0)))
    (else
      (Variables|Default|SetInteractable%20Actor 0))))