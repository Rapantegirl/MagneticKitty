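; BP_Door is a hinged door that opens and closes in response to a linked puzzle actor.
; On BeginPlay it binds to the OnSolvedChanged event of that actor's AC_PuzzleElement component, opening when solved and closing when unsolved.
; A timeline rotates DoorRoot's yaw to swing the door a quarter turn, playing to open and reversing to close.
; With OpensJustOnce set, it unbinds after the first solve and stays open.
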(event Custom|Open
  (bind _value (Timeline|Door%20Animation Play)
    (:Update
      (Transformation|SetRelativeRotation (Variables|Default|GetDoor%20Root) (Math|Rotator|MakeRotator 0.0 0.0 (Math|Float|Lerp 0.0 -9e+01 _value)) false false))))

(event Custom|Close
  (bind _value (Timeline|Door%20Animation Reverse)
    (:Update
      (Transformation|SetRelativeRotation (Variables|Default|GetDoor%20Root) (Math|Rotator|MakeRotator 0.0 0.0 (Math|Float|Lerp 0.0 -9e+01 _value)) false false))))

(event Custom|On%20Solved%20Changed_Event
  (params (Is%20Solved :type Boolean))
  (if Is%20Solved
    (if (Variables|Default|GetOpens%20just%20Once)
      (EventDispatchers|UnbindEventfromOnSolvedChanged (Actor|GetComponentbyClass (Variables|Default|GetPuzzle%20Actor) "/Game/Blueprints/interaction/AC_PuzzleElement.AC_PuzzleElement_C") (delegate Custom|On%20Solved%20Changed_Event)))
    (CallFunction|Open)
    (else
      (CallFunction|Close))))

(event EventBeginPlay
  (bind _puzzle_actor (Variables|Default|GetPuzzle%20Actor)
    (:then
      (Utilities|IsValid (Actor|GetComponentbyClass _puzzle_actor "/Game/Blueprints/interaction/AC_PuzzleElement.AC_PuzzleElement_C")
        (:Is%20Valid
          (EventDispatchers|AssignOnSolvedChanged (Actor|GetComponentbyClass _puzzle_actor "/Game/Blueprints/interaction/AC_PuzzleElement.AC_PuzzleElement_C") (delegate Custom|On%20Solved%20Changed_Event)))))
    (:else)))

(event Collision|EventActorBeginOverlap
  (params (OtherActor :type Actor%20Object%20Reference)))

(event EventTick
  (params (DeltaSeconds :type Float%20%28single-precision%29)))

(fn ConstructionScript)