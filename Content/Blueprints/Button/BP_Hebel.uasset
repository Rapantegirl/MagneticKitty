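; BP_Hebel is an interactable lever that toggles its puzzle element between solved and unsolved.
; Each interaction plays or reverses the ButtonAnimation timeline, which lerps ButtonRoot vertically.
; The timeline update also sets WegFrei on ZielBox and destroys the Blockade actor, in either direction, so reversing does not restore them.
; The construction script derives the timeline play rate from AnimationTimeInSeconds.
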(event EventBeginPlay)

(event Collision|EventActorBeginOverlap
  (params (OtherActor :type Actor%20Object%20Reference)))

(event EventTick
  (params (DeltaSeconds :type Float%20%28single-precision%29)))

(event EventOnInteract
  (bind _blockade (Variables|Default|GetBlockade))
  (if (Variables|/Game/Blueprints/interaction/AC_PuzzleElement.AC_PuzzleElement_C|GetSolved (Variables|Default|GetAC_PuzzleElement))
    (Default|SetPuzzleSolved (Variables|Default|GetAC_PuzzleElement) false)
    (bind _value (Timeline|Button%20Animation Reverse)
      (:Update
        (Transformation|SetRelativeLocation (Variables|Default|GetButton_Root) (Math|Vector|MakeVector 0.0 0.0 (Math|Float|Lerp 0.0 -12.0 _value)) false false)
        (Variables|/Game/Blueprints/Button/BP_Boxes.BP_Boxes_C|SetWegFrei (Variables|Default|GetZielBox) true)
        (Utilities|IsValid _blockade
          (:Is%20Valid
            (Actor|DestroyActor _blockade)))))
    (else
      (Default|SetPuzzleSolved (Variables|Default|GetAC_PuzzleElement) true)
      (Timeline|Button%20Animation Play))))

(fn ConstructionScript
  (Components|Timeline|SetPlayRate (Variables|Default|GetButton%20Animation) (/ 1.0 (Variables|Default|GetAnimation%20Time%20in%20Seconds))))