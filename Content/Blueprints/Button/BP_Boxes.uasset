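; BP_Boxes is an interactable box actor that moves one step along a list of target transforms per interaction, opening a door at the last one.
; On interact, if the WegFrei flag is set, the Bewegung timeline lerps it from its current transform to the next TeleportZiele entry without sweeping.
; When the timeline finishes, the step counter increments and ZielDoor opens after the final target.
; If the path is not free, it prints a German "blocked" message.
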(event EventBeginPlay)

(event Collision|EventActorBeginOverlap
  (params (OtherActor :type Actor%20Object%20Reference)))

(event EventTick
  (params (DeltaSeconds :type Float%20%28single-precision%29)))

(event EventOnInteract
  (if (Variables|Default|GetWegFrei)
    (if (< (Variables|Default|GetAktueller%20Schritt) (Utilities|Array|Length (Variables|Default|GetTeleportZiele)))
      (Variables|Default|SetStartPosition (Transformation|GetActorTransform))
      (Variables|Default|SetZielPosition (Utilities|Array|Get(acopy) (Variables|Default|GetTeleportZiele) (Variables|Default|GetAktueller%20Schritt)))
      (bind _alpha (Timeline|Bewegung PlayFromStart)
        (:Update
          (Transformation|SetActorTransform (Math|Transform|Lerp(Transform) (Variables|Default|GetStartPosition) (Variables|Default|GetZielPosition) _alpha)))
        (:Finished
          (Variables|Default|SetAktueller%20Schritt (+ (Variables|Default|GetAktueller%20Schritt) 1))
          (if (== (Variables|Default|GetAktueller%20Schritt) (Utilities|Array|Length (Variables|Default|GetTeleportZiele)))
            (Default|Open (Variables|Default|GetZielDoor))))))
    (else
      (Development|PrintString "Der Weg ist versperrt!"))))

(fn ConstructionScript)